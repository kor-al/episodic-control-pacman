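; BP_PacDotActor is a Pac-Man dot pickup that serves as either a regular dot or a power-up, selected by ISPowerUp.
; On overlap with BP_PacManPawn, a power-up calls the pawn's EatGhostEvent, while a regular dot updates the score through BP_GameMode; both then destroy themselves.
; The construction script recolors and rescales power-up dots.
; An unconnected node setting the game mode's WasPowered never runs.
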(event Collision|EventActorBeginOverlap
  (params (OtherActor :type Actor%20Object%20Reference))
  (bind _asbp_pac_man_pawn (Utilities|Casting|CastToBP_PacManPawn OtherActor))
  (if (Variables|Default|GetISPowerUp?)
    (Default|EatGhostEvent _asbp_pac_man_pawn)
    (else
      (bind _asbp_game_mode (Utilities|Casting|CastToBP_GameMode (Game|GetGameMode)))
      (Default|UpdatePlayerScore _asbp_game_mode)))
  (Actor|DestroyActor))

(fn ConstructionScript
  (if (Variables|Default|GetISPowerUp?)
    (Sprite|SetSpriteColor (Variables|Default|GetPacDot_Sprite) "(R=1.000000,G=0.119107,B=0.013846,A=1.000000)")
    (Transformation|SetWorldScale3D "0.600000,0.600000,0.600000")))