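; Pac-Man-style ghost character in five color types, which roams between destination points and switches between dangerous, edible and eaten states.
; FindNextDestination claims a random untaken BP_GhostDestinationPoint, excluding the current one, and retries failed AI moves.
; Timers move edible ghosts through flashing back to normal, while eaten ghosts head to their start location.
; Tick selects directional, frightened or eyes-only flipbooks from state and velocity, using a per-color animation struct.
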(event Custom|CanBeEatenEvent
  (if (not (Variables|Default|GetIsDead?))
    (Utilities|Time|ClearandInvalidateTimerbyHandle (Variables|Default|GetFlashingEventTimerHandle))
    (Utilities|Time|ClearandInvalidateTimerbyHandle (Variables|Default|GetBackToNormalTimerHandle))
    (Variables|/Script/Engine.CharacterMovementComponent|SetMaxWalkSpeed (Variables|Character|GetCharacterMovement) 3e+02)
    (Variables|Default|SetCanKill false)
    (Variables|Default|SetCanBeEaten true)
    (Variables|Default|SetIsFlasing false)
    (bind _returnvalue (Utilities|Time|SetTimerbyFunctionName self "FlashingEvent" (Variables|Default|GetCanBeEatenTime)))
    (Variables|Default|SetFlashingEventTimerHandle _returnvalue)))

(event Custom|FlashingEvent
  (Variables|Default|SetIsFlasing true)
  (Utilities|Time|SetTimerbyFunctionName self "BackToNormal" (Variables|Default|GetFlashingTime)))

(event Custom|BackToStart
  (Transformation|SetActorLocation (Variables|Default|GetStartLocation) false true)
  (CallFunction|BacktoNormal))

(event Custom|BackToNormal
  (Variables|Default|SetIsDead? false)
  (Variables|Default|SetCanBeEaten false)
  (Variables|Default|SetIsFlasing false)
  (Variables|Default|SetCanKill true)
  (Variables|/Script/Engine.CharacterMovementComponent|SetMaxWalkSpeed (Variables|Character|GetCharacterMovement) 4e+02))

(event Custom|FindNextDestination
  (Utilities|IsValid (Variables|Default|GetCurrentTarget%20Trigger)
    (:Is%20Valid
      (bind _outactors (Actor|GetAllActorsOfClass "/Game/Blueprints/BP_GhostDestinationPoint.BP_GhostDestinationPoint_C"))
      (Variables|Default|SetTargetTriggers_Array_Temp _outactors)
      (Utilities|Array|RemoveItem (Variables|Default|GetTargetTriggers_Array_Temp) (Variables|Default|GetCurrentTarget%20Trigger)))
    (:Is%20Not%20Valid
      (bind _outactors_2 (Actor|GetAllActorsOfClass "/Game/Blueprints/BP_GhostDestinationPoint.BP_GhostDestinationPoint_C"))
      (Variables|Default|SetTargetTriggers_Array_Temp _outactors_2)))
  (for _array_element (Variables|Default|GetTargetTriggers_Array_Temp)
    (if (Variables|/Game/Blueprints/BP_GhostDestinationPoint.BP_GhostDestinationPoint_C|GetIsTaken _array_element)
      (Utilities|Array|RemoveItem (Variables|Default|GetTargetTriggers_Array_Temp) _array_element)))
  (Variables|Default|SetCurrentTarget%20Trigger (Utilities|Array|Get(acopy) (Variables|Default|GetTargetTriggers_Array_Temp) (Math|Random|RandomIntegerinRange 0 (- (Utilities|Array|Length (Variables|Default|GetTargetTriggers_Array_Temp)) 1))))
  (Variables|/Game/Blueprints/BP_GhostDestinationPoint.BP_GhostDestinationPoint_C|SetIsTaken (Variables|Default|GetCurrentTarget%20Trigger) true)
  (AI|AIMoveTo self "0, 0, 0" (Variables|Default|GetCurrentTarget%20Trigger) 5.0 false :!label _label
    (:OnFail
      (Utilities|FlowControl|Delay 0.2 :!label _label_2)
      (if (Variables|Default|GetIsDead?)
        (Utilities|FlowControl|Delay 0.2)
        (goto _label_2)
        (else
          (goto _label))))))

(event Custom|EatEvent
  (if (and (Variables|Default|GetCanBeEaten) (not (Variables|Default|GetIsDead?)))
    (Utilities|Time|ClearandInvalidateTimerbyHandle (Variables|Default|GetFlashingEventTimerHandle))
    (Utilities|Time|ClearandInvalidateTimerbyHandle (Variables|Default|GetBackToNormalTimerHandle))
    (Variables|Default|SetCanBeEaten false)
    (Variables|Default|SetIsDead? true)
    (AI|Navigation|SimpleMovetoLocation (Pawn|GetController) (Variables|Default|GetStartLocation))
    (Variables|/Script/Engine.CharacterMovementComponent|SetMaxWalkSpeed (Variables|Character|GetCharacterMovement) 4e+02)))

(event Custom|Reset
  (Variables|Default|SetCanBeEaten true)
  (Variables|Default|SetIsFlasing true)
  (Utilities|FlowControl|Delay 1.0)
  (CallFunction|BacktoNormal)
  (CallFunction|FindNextDestination))

(event EventBeginPlay
  (Variables|Default|SetStartLocation (Transformation|GetActorLocation))
  (CallFunction|BacktoNormal)
  (switch Utilities|FlowControl|Switch|SwitchonEnum_GhostType (Variables|Default|GetType)
    (:NewEnumerator1
      (|SetRedAnimations (Variables|Default|GetAnimationsStruct)))
    (:NewEnumerator2
      (|SetCyanAnimations (Variables|Default|GetAnimationsStruct)))
    (:NewEnumerator3
      (|SetYellowAnimations (Variables|Default|GetAnimationsStruct)))
    (:NewEnumerator4
      (|SetGreenAnimations (Variables|Default|GetAnimationsStruct)))
    (:NewEnumerator5
      (|SetPinkAnimations (Variables|Default|GetAnimationsStruct)))))

(event EventTick
  (params (DeltaSeconds :type Float%20%28single-precision%29))
  (bind (_normal _dead) (|MoveRightAnimations))
  (bind (_normal_2 _dead_2) (|MoveLeftAnimations))
  (bind (_blue _flashing) (|CanBeEatenAnimations))
  (bind (_normal_3 _dead_3) (|MoveUpAnimations))
  (bind (_normal_4 _dead_4) (|MoveDownAnimations))
  (|CheckIfCanBeEaten
    (:True
      (Sprite|SetFlipbook (Variables|Default|GetSprite) (select (Variables|Default|GetIsFlasing) _flashing _blue)))
    (:False
      (|StoringTempVelocity)
      (|CheckIfIsMovingVertically
        (:True
          (|CheckIfIsMovingUP
            (:True
              (Sprite|SetFlipbook (Variables|Default|GetSprite) (select (Variables|Default|GetIsDead?) _dead_3 _normal_3)))
            (:False
              (Sprite|SetFlipbook (Variables|Default|GetSprite) (select (Variables|Default|GetIsDead?) _dead_4 _normal_4)))))
        (:False
          (|CheckIfIsMovingRight
            (:True
              (Sprite|SetFlipbook (Variables|Default|GetSprite) (select (Variables|Default|GetIsDead?) _dead _normal)))
            (:False
              (Sprite|SetFlipbook (Variables|Default|GetSprite) (select (Variables|Default|GetIsDead?) _dead_2 _normal_2)))))))))

(fn ConstructionScript
  (switch Utilities|FlowControl|Switch|SwitchonEnum_GhostType (Variables|Default|GetType)
    (:NewEnumerator1
      (Sprite|SetFlipbook (Variables|Default|GetSprite) "/Game/FlipBooks/Red_U.Red_U"))
    (:NewEnumerator2
      (Sprite|SetFlipbook (Variables|Default|GetSprite) "/Game/FlipBooks/Cyan_U.Cyan_U"))
    (:NewEnumerator3
      (Sprite|SetFlipbook (Variables|Default|GetSprite) "/Game/FlipBooks/Yellow_U.Yellow_U"))
    (:NewEnumerator4
      (Sprite|SetFlipbook (Variables|Default|GetSprite) "/Game/FlipBooks/Green_U.Green_U"))
    (:NewEnumerator5
      (Sprite|SetFlipbook (Variables|Default|GetSprite) "/Game/FlipBooks/Pink_U.Pink_U"))))