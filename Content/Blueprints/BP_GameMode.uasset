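; Game mode for a Pac-Man game that runs the board, score and episode state.
; BeginPlay spawns the block grid, starts ghost pathing, creates a screen capturer, increments the GameInstance episode count and spawns Pac-Man at a PlayerStart.
; Helpers map world positions to grid blocks, and dot destruction triggers the win check.
; Events update score and flag episode end on death; ResetDots respawns saved transforms, but the saving logic is unwired.
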(event Custom|DeathScoreUpdate
  (Variables|/Script/PacMan.PacGameInstance|SetisEpisodeEnded (Variables|Default|GetPacGameInstRef) true))

(event Custom|WinEvent
  (params (DestroyedActor :type Actor%20Object%20Reference))
  (bind _outactors (Actor|GetAllActorsOfClass "/Game/Blueprints/BP_PacDotActor.BP_PacDotActor_C"))
  (if (== (Utilities|Array|Length _outactors) 1)
    (Development|PrintString "You Won")))

(event Custom|Update%20Player%20Score%20Ghost
  (Variables|Default|SetPlayer_Score (+ 200 (Variables|Default|GetPlayer_Score))))

(event Custom|ResetDots
  (for (_array_element _array_index) (Variables|Default|GetDotsTranformArray)
    (bind _returnvalue (Game|SpawnActorfromClass "/Game/Blueprints/BP_PacDotActor.BP_PacDotActor_C" _array_element "Undefined" 0 0)))
  (Utilities|Array|Clear (Variables|Default|GetDotsTranformArray))
  (Utilities|Array|Clear (Variables|Default|GetPoweredDestroyedDotsArray)))

(event Custom|Reset%20Player%20Score
  (Variables|Default|SetPlayer_Score 0))

(event Custom|SpawnPacMan
  (bind _outactors (Actor|GetAllActorsOfClass "/Script/Engine.PlayerStart"))
  (Game|SpawnActorfromClass "/Game/Blueprints/BP_PacManPawn.BP_PacManPawn_C" (Transformation|GetActorTransform (Utilities|Array|Get(acopy) _outactors)) "AlwaysSpawn" 0 0))

(event Custom|Update%20Player%20Score
  (bind _result (Math|Integer|IncrementInt (Variables|Default|GetPlayer_Score))
    (:%20%20
      (Variables|Default|SetPlayer_Score _result))))

(event Custom|CreateGrid
  (Utilities|Array|Clear (Variables|Default|GetBlocksArray))
  (for _index (range 0 (- (* (Variables|Default|GetMax%20X) (Variables|Default|GetMax%20Y)) 1))
    (bind _returnvalue (Game|SpawnActorfromClass "/Game/Blueprints/BP_GridBlockActor.BP_GridBlockActor_C" (Math|Transform|MakeTransform (Math|Vector|MakeVector (* (/ _index 21) (Variables|Default|GetSpacing)) (* (Math|Integer|%(Integer) _index 21) (Variables|Default|GetSpacing)) 0.0) "0, 0, 0" "1,1,1") "AlwaysSpawn" 0 0))
    (Utilities|Array|Add (Variables|Default|GetBlocksArray) _returnvalue)
    (bind _outactors (Actor|GetAllActorsOfClass "/Game/Blueprints/BP_PacDotActor.BP_PacDotActor_C"))
    (for _array_element _outactors
      (Game|BindEventtoOnDestroyed _array_element (delegate Custom|WinEvent)))))

(event EventBeginPlay
  (CallFunction|CreateGrid)
  (bind _outactors (Actor|GetAllActorsOfClass "/Game/Blueprints/BP_GhostCharacter.BP_GhostCharacter_C"))
  (for _array_element _outactors
    (Default|FindNextDestination _array_element))
  (bind _returnvalue (Game|SpawnActorfromClass "/Game/Blueprints/ScreenCapturer_BP.ScreenCapturer_BP_C" (Math|Transform|MakeTransform "0, 0, 0") "Undefined" 0 0))
  (Variables|Default|SetScreenCapturer _returnvalue)
  (bind _asbp_pac_game_instance (Utilities|Casting|CastToBP_PacGameInstance (Game|GetGameInstance)))
  (Variables|Default|SetPacGameInstRef _asbp_pac_game_instance)
  (Math|Integer|IncrementInt (Variables|/Script/PacMan.PacGameInstance|GetEpisodesNum _asbp_pac_game_instance)
    (:%20%20
      (CallFunction|SpawnPacMan))))

(fn ConstructionScript)

(fn WorldtoGridLocation
  (params (Location :type Vector))
  (bind _spacing (Variables|Default|GetSpacing))
  (bind _spacing_2 (Variables|Default|GetSpacing))
  (return (Math|Integer|Clamp(Integer) (Math|Float|Floor (/ (+ (.x Location) (/ _spacing_2 2.0)) _spacing_2)) 0 (- (Variables|Default|GetMax%20X) 1)) (Math|Integer|Clamp(Integer) (Math|Float|Floor (/ (+ (.y Location) (/ _spacing 2.0)) _spacing)) 0 (- (Variables|Default|GetMax%20Y) 1))))

(fn GetBlockfromGridLocation
  (params (X :type Integer :default 0) (Y :type Integer :default 0))
  (return (Utilities|Array|Get(acopy) (Variables|Default|GetBlocksArray) (+ (* X (Variables|Default|GetMax%20Y)) (Math|Integer|%(Integer) Y (Variables|Default|GetMax%20Y))))))

(fn GetBlockfromWorldLocation
  (params (Location :type Vector :default "0, 0, 0"))
  (bind (_x _y) (CallFunction|WorldtoGridLocation Location))
  (bind _blockactor (CallFunction|GetBlockfromGridLocation _x _y))
  (return _blockactor))