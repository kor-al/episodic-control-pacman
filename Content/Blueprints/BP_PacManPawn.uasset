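; Pac-Man player pawn that moves cell by cell on the game mode's grid, steered by an integer Action.
; After skipping initial frames, Tick checks walkable blocks, updates the flipbook and lerps one cell via timeline, gated by a resettable DoOnce.
; Ghost overlaps either eat the ghost for score or trigger death, destruction and a level reload; EatGhostEvent makes all ghosts edible.
; Keyboard steering and an older movement chain remain disconnected.
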(event Custom|EatGhostEvent
  ;[1 1 1] Eat Ghost Event
  (bind _outactors (Actor|GetAllActorsOfClass "/Game/Blueprints/BP_GhostCharacter.BP_GhostCharacter_C"))
  (for _array_element _outactors
    (Default|CanbeEatenEvent _array_element)))

(event Custom|ResetDoOnce
  ;[1 1 1] Tick_1 Event
  (Utilities|FlowControl|DoOnce false) ; enters at Reset
)

(event Custom|RespawnEvent
  (params (DestroyedActor :type Actor%20Object%20Reference))
  ;[1 1 0] Respawn Event ( Called When PacManPawn_BP is Destroyed)
  (Default|DeathScoreUpdate (Variables|Default|GetGameModeRef))
  (Game|OpenLevel(byName) "Map_Example"))

(event Custom|MakeInvisible
  (Development|SetHiddeninGame (Variables|Default|GetPacMan_FlipBook) false false))

(event Collision|EventActorBeginOverlap
  (params (OtherActor :type Actor%20Object%20Reference))
  ;[1 1 1] PacMan/Ghost Collision Event
  (bind _asbp_ghost_character (Utilities|Casting|CastToBP_GhostCharacter OtherActor))
  (if (and (not (Variables|Default|GetIsDead?)) (Variables|/Game/Blueprints/BP_GhostCharacter.BP_GhostCharacter_C|GetCanKill _asbp_ghost_character))
    (Variables|Default|SetIsDead? true)
    (else
      (Default|EatEvent _asbp_ghost_character)
      (Default|UpdatePlayerScoreGhost (Variables|Default|GetGameModeRef)))))

(event EventTick
  (params (DeltaSeconds :type Float%20%28single-precision%29))
  (bind _ticknum (Variables|Default|GetTickNum))
  (if (Variables|Default|GetareFirstFramesSkipped?)
    ;[1 1 1] Tick_1 Event
    (if (Variables|Default|GetIsDead?) :!label _label
      (Utilities|FlowControl|DoOnce false
        (:Completed
          ;;[1 0 0] Death Sequence
          (Utilities|FlowControl|Delay 0.2) ; Wait 0.2 Sec
          (CallFunction|UpdateAnimation)
          (Utilities|FlowControl|Delay 1.0) ; Wait 1 Sec
          (Actor|DestroyActor) ; Kill PacMan
        ))
      (else
        (Utilities|FlowControl|DoOnce false
          (:Completed
            ;;[0 1 0.5763] Store PacMan Current Location
            (Variables|Default|SetTempLocation (Transformation|GetWorldLocation))
            ;;[1 0.09459 0] Check Collision
            (|CheckRightCollision_2
              (:True
                (Variables|Default|SetDirection%20X 0))
              (:else
                (|CheckLeftCollision_2
                  (:True
                    (Variables|Default|SetDirection%20X 0))
                  (:else
                    (|CheckUpCollision_2
                      (:True
                        (Variables|Default|SetDirection%20Y 0))
                      (:else
                        (|CheckDownCollision_2
                          (:True
                            (Variables|Default|SetDirection%20Y 0))
                          (:Else
                            _))))))))
            ;;[0.09255 1 0.3687] AI movement
            (switch int (Variables|Default|Getaction)
              (:Default
                _)
              (:1
                (bind (_x _y) (Default|WorldtoGridLocation (Variables|Default|GetGameModeRef) (Transformation|GetActorLocation)))
                (bind _blockactor (Default|GetBlockfromGridLocation (Variables|Default|GetGameModeRef) (+ _x 1) _y))
                (if (and (Variables|/Game/Blueprints/BP_GridBlockActor.BP_GridBlockActor_C|GetIsWalkables _blockactor) (Variables|Default|GetCanChangeDirection))
                  (Variables|Default|SetDirection%20X 1)
                  (Variables|Default|SetDirection%20Y 0)))
              (:2
                (bind (_x_2 _y_2) (Default|WorldtoGridLocation (Variables|Default|GetGameModeRef) (Transformation|GetActorLocation)))
                (bind _blockactor_2 (Default|GetBlockfromGridLocation (Variables|Default|GetGameModeRef) _x_2 (+ _y_2 1)))
                (if (and (Variables|/Game/Blueprints/BP_GridBlockActor.BP_GridBlockActor_C|GetIsWalkables _blockactor_2) (Variables|Default|GetCanChangeDirection))
                  (Variables|Default|SetDirection%20Y 1)
                  (Variables|Default|SetDirection%20X 0)))
              (:3
                (bind (_x_3 _y_3) (Default|WorldtoGridLocation (Variables|Default|GetGameModeRef) (Transformation|GetActorLocation)))
                (bind _blockactor_3 (Default|GetBlockfromGridLocation (Variables|Default|GetGameModeRef) (+ _x_3 -1) _y_3))
                (if (and (Variables|/Game/Blueprints/BP_GridBlockActor.BP_GridBlockActor_C|GetIsWalkables _blockactor_3) (Variables|Default|GetCanChangeDirection))
                  (Variables|Default|SetDirection%20X -1)
                  (Variables|Default|SetDirection%20Y 0)))
              (:4
                (bind (_x_4 _y_4) (Default|WorldtoGridLocation (Variables|Default|GetGameModeRef) (Transformation|GetActorLocation)))
                (bind _blockactor_4 (Default|GetBlockfromGridLocation (Variables|Default|GetGameModeRef) _x_4 (+ _y_4 -1)))
                (if (and (Variables|/Game/Blueprints/BP_GridBlockActor.BP_GridBlockActor_C|GetIsWalkables _blockactor_4) (Variables|Default|GetCanChangeDirection))
                  (Variables|Default|SetDirection%20Y -1)
                  (Variables|Default|SetDirection%20X 0))))
            ;;[1 0 0.8631] Update Anamiation
            (CallFunction|UpdateAnimation)
            ;;[0 0.001349 0.26] Movement Update
            (if (or (!= (Variables|Default|GetDirection%20X) 0) (!= (Variables|Default|GetDirection%20Y) 0))
              (bind _lerppercent (Timeline|Timeline_0 PlayFromStart)
                (:Update
                  (Transformation|SetWorldLocation (Math|Vector|Lerp(Vector) (Variables|Default|GetTempLocation) (+ (Variables|Default|GetTempLocation) (Math|Vector|MakeVector (* (Variables|Default|GetDirection%20X) 1e+02) (* (Variables|Default|GetDirection%20Y) 1e+02) 0.0)) _lerppercent) false false))
                (:Finished
                  ;;[0 0.6682 1] Reset Do  Once Event
                  (CallFunction|ResetDoOnce :!label _label_2)))
              (else
                (goto _label_2)))))))
    (else
      (Math|Integer|IncrementInt _ticknum
        (:%20%20
          (if (>= _ticknum 3)
            (Variables|Default|SetareFirstFramesSkipped? true)
            (goto _label)))))))

(event EventBeginPlay
  ;[1 1 1] Begin Play Event
  (Variables|Default|SetIsDead? false)
  (bind _asbp_game_mode (Utilities|Casting|CastToBP_GameMode (Game|GetGameMode)))
  (Variables|Default|SetGameModeRef _asbp_game_mode)
  (Variables|Default|SetpGameMode _asbp_game_mode)
  (EventDispatchers|BindEventtoOnDestroyed (delegate Custom|RespawnEvent)))

(fn ConstructionScript)

(fn UpdateAnimation
  (if (Variables|Default|GetIsDead?)
    (Sprite|SetFlipbook (Variables|Default|GetPacMan_FlipBook) "/Game/FlipBooks/PacDeath_Flipbook.PacDeath_Flipbook")
    (else
      (if (== (Variables|Default|GetDirection%20X) 1)
        (LocalVariables|SetTempYaw 1.8e+02)
        (Sprite|SetFlipbook (Variables|Default|GetPacMan_FlipBook) "/Game/FlipBooks/PacMan_Walk.PacMan_Walk" :!label _label)
        (elif (== (Variables|Default|GetDirection%20X) -1)
          (LocalVariables|SetTempYaw 0.0)
          (goto _label)
          (elif (== (Variables|Default|GetDirection%20Y) 1)
            (LocalVariables|SetTempYaw 2.7e+02)
            (goto _label)
            (elif (== (Variables|Default|GetDirection%20Y) -1)
              (LocalVariables|SetTempYaw 9e+01)
              (goto _label)
              (else
                (Sprite|SetFlipbook (Variables|Default|GetPacMan_FlipBook) "/Game/FlipBooks/PacManBlocked.PacManBlocked"))))))
      (Transformation|SetRelativeRotation (Variables|Default|GetPacMan_FlipBook) (Math|Rotator|MakeRotator -9e+01 0.0 (LocalVariables|GetTempYaw)) false false)))
  (return))

(event Input|KeyboardEvents|Right
  (params (Key :type Key%20Structure :default "AnyKey"))
  (:Pressed
    (Utilities|FlowControl|Gate true) ; enters at Open
  )
  (:Released
    (Utilities|FlowControl|Gate true) ; enters at Close
  ))

(event Input|KeyboardEvents|Left
  (params (Key :type Key%20Structure :default "AnyKey"))
  (:Pressed
    (Utilities|FlowControl|Gate true) ; enters at Open
  )
  (:Released
    (Utilities|FlowControl|Gate true) ; enters at Close
  ))

(event Input|KeyboardEvents|Up
  (params (Key :type Key%20Structure :default "AnyKey"))
  (:Pressed
    (Utilities|FlowControl|Gate true) ; enters at Open
  )
  (:Released
    (Utilities|FlowControl|Gate true) ; enters at Close
  ))

(event Input|KeyboardEvents|Down
  (params (Key :type Key%20Structure :default "AnyKey"))
  (:Pressed
    (Utilities|FlowControl|Gate true) ; enters at Open
  )
  (:Released
    (Utilities|FlowControl|Gate true) ; enters at Close
  ))